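; BP_WinVolume is a level-exit trigger that advances the game once every BP_crystal02 actor is gone from the level.
; On box overlap, with no check on the overlapping actor, it prints a Polish warning if crystals remain, otherwise fades to opaque and calls Completelevel after a delay.
; Completelevel finds the current level in TabLevelNames and opens the next entry, or only prints a message on the final level.
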(event OnComponentBeginOverlap(Box)
  (params (OverlappedComponent :type Primitive%20Component%20Object%20Reference) (OtherActor :type Actor%20Object%20Reference) (OtherComp :type Primitive%20Component%20Object%20Reference) (OtherBodyIndex :type Integer) (bFromSweep :type Boolean) (SweepResult :type Hit%20Result%20Structure%20%28by%20ref%29))
  (bind _outactors (Actor|GetAllActorsOfClass "/Game/blueprints/crystals/BP_crystal02.BP_crystal02_C"))
  (if (> (Utilities|Array|Length _outactors) 0)
    (Development|PrintString "Nie zebrano wszystkich kryształów")
    (else
      (CameraFades|StartCameraFade :self (Game|GetPlayerCameraManager 0) :FromAlpha 0.0 :ToAlpha 1.0 :Duration 1.0 :bHoldWhenFinished true)
      (Utilities|FlowControl|Delay 1.0)
      (CallFunction|Completelevel))))

(fn ConstructionScript)

(fn GetCurrentLevelIndex
  (bind _returnvalue (Game|GetCurrentLevelName true))
  (return (Utilities|Array|FindItem (Variables|Default|GetTab_level_names) _returnvalue)))

(fn GetNextLevelName
  (return (Utilities|Array|Get(acopy) (Variables|Default|GetTab_level_names) (+ (CallFunction|GetCurrentLevelIndex) 1))))

(fn LoadNextLevel
  (Game|OpenLevel(byName) (Utilities|String|StringToName (CallFunction|GetNextLevelName))))

(fn IsFinalLevel
  (return (== (Utilities|Array|LastIndex (Variables|Default|GetTab_level_names)) (CallFunction|GetCurrentLevelIndex))))

(fn Completelevel
  (if (CallFunction|IsFinalLevel)
    (Development|PrintString "to jest ostatni poziom")
    (else
      (CallFunction|LoadNextLevel))))