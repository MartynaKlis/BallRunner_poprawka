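; BP_crystal02 is a collectible crystal pickup that triggers when the player pawn overlaps its sphere.
; A timeline lerps the crystal from its current location toward the player pawn while shrinking its scale to zero.
; The point light intensity is also lerped each update, but its alpha is fixed at zero, so it never dims.
; When the timeline finishes, it plays a 2D collect sound and destroys the actor.
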(event OnComponentBeginOverlap(Sphere)
  (params (OverlappedComponent :type Primitive%20Component%20Object%20Reference) (OtherActor :type Actor%20Object%20Reference) (OtherComp :type Primitive%20Component%20Object%20Reference) (OtherBodyIndex :type Integer) (bFromSweep :type Boolean) (SweepResult :type Hit%20Result%20Structure%20%28by%20ref%29))
  (bind _pointlight (Variables|Default|GetPointLight))
  (Utilities|IsPlayer OtherActor)
  (bind (_direction _transform_location _transform_scale) (Timeline|Crystal_Transforms_01 Play)
    (:Update
      (Transformation|SetActorLocation (Math|Vector|Lerp(Vector) (Transformation|GetActorLocation) (Transformation|GetActorLocation (Game|Player|GetPlayerPawn 0)) _transform_location) false false)
      (Transformation|SetActorScale3D (Math|Vector|Lerp(Vector) (Transformation|GetActorScale3D) "0, 0, 0" _transform_scale))
      (Variables|Default|SetIntensity (Variables|/Script/Engine.LightComponentBase|GetIntensity _pointlight))
      (Rendering|Components|Light|SetIntensity _pointlight (Math|Float|Lerp (Variables|Default|GetIntensity) 0.0 0.0)))
    (:Finished
      (Audio|PlaySound2D "/Game/sounds/Collect_Item_Sound_Effect-yt_savetube_me.Collect_Item_Sound_Effect-yt_savetube_me" 1.0 1.0 0.0 0 0)
      (Actor|DestroyActor))))

(event EventBeginPlay)

(event Collision|EventActorBeginOverlap
  (params (OtherActor :type Actor%20Object%20Reference)))

(fn ConstructionScript)